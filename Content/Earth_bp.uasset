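; Earth Blueprint actor that spins on its axis and circles the world origin, with Velocity acting as a time scale.
; Each Tick, a collapsed graph adds local yaw at one turn per 86400-second day, scaled by Velocity.
; Tick then accumulates time in Translate and sets an XY position from sine and cosine at radius Distance.
; The orbit angle divides scaled time by a year's seconds without a 2π factor.
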(event `self.ReceiveTick`
  (params (DeltaSeconds :type "Float (single-precision)"))
  (bind _distance (`self.Distance`))
  (`|ExecutionSequence`
    (:`then_0`
      (`self.K2_AddActorLocalRotation` (`KismetMathLibrary.MakeRotator` 0.0 0.0 (* DeltaSeconds (/ (* (`self.Velocity`) 360.0) 86400.0)))))
    (:`then_1`
      (bind _output_get (set `self.Translate` (+ DeltaSeconds (`self.Translate`))))
      (bind _returnvalue (/ (* _output_get (`self.Velocity`)) 31536000.0))
      (`self.K2_SetActorLocation` (`KismetMathLibrary.MakeVector` (* (`KismetMathLibrary.Sin` _returnvalue) _distance) (* (`KismetMathLibrary.Cos` _returnvalue) _distance))))))

(fn `UserConstructionScript`)